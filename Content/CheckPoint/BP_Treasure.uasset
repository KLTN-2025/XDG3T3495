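; BP_Treasure is a treasure actor that rises and lights up when something overlaps its Box.
; The Goup timeline lerps its Z from the current location toward Height with sweep.
; A delay off that timeline's update starts the Lightup timeline, which ramps the PointLight intensity up sharply.
; The overlap also adds a WB_flash widget after its own delay; the widget removal logic is unconnected.
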(event OnComponentBeginOverlap(Box)
  (params (OverlappedComponent :type Primitive%20Component%20Object%20Reference) (OtherActor :type Actor%20Object%20Reference) (OtherComp :type Primitive%20Component%20Object%20Reference) (OtherBodyIndex :type Integer) (bFromSweep :type Boolean) (SweepResult :type Hit%20Result%20Structure%20%28by%20ref%29))
  (CallFunction|GOUp)
  (Utilities|FlowControl|Delay 11.0)
  (bind _returnvalue (UserInterface|CreateWidget "/Game/UI/WB_flash.WB_flash_C"))
  (UserInterface|Viewport|AddtoViewport _returnvalue 0))

(event Custom|GO%20up
  (bind _returnvalue (Transformation|GetActorLocation))
  (bind _alpha (Timeline|goup PlayFromStart)
    (:Update
      (Transformation|SetActorLocation (Math|Vector|Lerp(Vector) _returnvalue (Math|Vector|MakeVector (.X (Math|Vector|BreakVector _returnvalue)) (.Y (Math|Vector|BreakVector _returnvalue)) (Variables|Default|GetHeight)) _alpha) true false)
      (Utilities|FlowControl|Delay 1e+01)
      (bind _alpha_2 (Timeline|lightup Play)
        (:Update
          (Rendering|Components|Light|SetIntensity (Variables|Default|GetPointLight) (Math|Float|Lerp 1e+02 1e+05 _alpha_2)))))))

(event EventBeginPlay)

(event Collision|EventActorBeginOverlap
  (params (OtherActor :type Actor%20Object%20Reference)))

(event EventTick
  (params (DeltaSeconds :type Float%20%28single-precision%29)))

(fn ConstructionScript)