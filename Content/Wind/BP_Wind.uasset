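; BP_Wind is a moving wind actor that travels in a straight line from where it starts and disappears on contact.
; On BeginPlay it stores its location and a Timeline lerps it a fixed distance along world +Y, without sweeping.
; An overlap on its Box component destroys the actor; the IsHit flag is set on first hit, though both branches destroy it.
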(event OnComponentBeginOverlap(Box)
  (params (OverlappedComponent :type Primitive%20Component%20Object%20Reference) (OtherActor :type Actor%20Object%20Reference) (OtherComp :type Primitive%20Component%20Object%20Reference) (OtherBodyIndex :type Integer) (bFromSweep :type Boolean) (SweepResult :type Hit%20Result%20Structure%20%28by%20ref%29))
  (if (Variables|Default|GetIsHit)
    (Actor|DestroyActor)
    (else
      (Variables|Default|SetIsHit true)
      (Actor|DestroyActor))))

(event EventBeginPlay
  (Variables|Default|SetstartLocation (Transformation|GetActorLocation))
  (Variables|Default|SetendLocation (Math|Vector|MakeVector (.X (Math|Vector|BreakVector (Variables|Default|GetstartLocation))) (+ (.Y (Math|Vector|BreakVector (Variables|Default|GetstartLocation))) 2e+03) (.Z (Math|Vector|BreakVector (Variables|Default|GetstartLocation)))))
  (bind _run (Timeline|Timeline Play)
    (:Update
      (Transformation|SetActorLocation (Math|Vector|Lerp(Vector) (Variables|Default|GetstartLocation) (Variables|Default|GetendLocation) _run) false false))))

(event Collision|EventActorBeginOverlap
  (params (OtherActor :type Actor%20Object%20Reference)))

(event EventTick
  (params (DeltaSeconds :type Float%20%28single-precision%29)))

(fn ConstructionScript)