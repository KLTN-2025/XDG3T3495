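; Bow actor that the third-person character can interact with while standing inside its Box trigger.
; Overlap sets the character's CurrentBow to this actor and end overlap clears it, each printing a debug message; the IsAiming branch rewrites the same value.
; A Hide event flips the IsHiden flag but hides the actor on both branches, so it never shows it again.
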(event OnComponentBeginOverlap(Box)
  (params (OverlappedComponent :type Primitive%20Component%20Object%20Reference) (OtherActor :type Actor%20Object%20Reference) (OtherComp :type Primitive%20Component%20Object%20Reference) (OtherBodyIndex :type Integer) (bFromSweep :type Boolean) (SweepResult :type Hit%20Result%20Structure%20%28by%20ref%29))
  (bind _asbp_third_person_character (Utilities|Casting|CastToBP_ThirdPersonCharacter OtherActor))
  (Variables|/Game/ThirdPerson/Blueprints/BP_ThirdPersonCharacter.BP_ThirdPersonCharacter_C|SetCurrentBow _asbp_third_person_character self)
  (Development|PrintString "can interact")
  (if (Variables|/Game/ThirdPerson/Blueprints/BP_ThirdPersonCharacter.BP_ThirdPersonCharacter_C|GetisAiming? _asbp_third_person_character)
    (Variables|/Game/ThirdPerson/Blueprints/BP_ThirdPersonCharacter.BP_ThirdPersonCharacter_C|SetisAiming? _asbp_third_person_character true)
    (else
      (Variables|/Game/ThirdPerson/Blueprints/BP_ThirdPersonCharacter.BP_ThirdPersonCharacter_C|SetisAiming? _asbp_third_person_character false))))

(event OnComponentEndOverlap(Box)
  (params (OverlappedComponent :type Primitive%20Component%20Object%20Reference) (OtherActor :type Actor%20Object%20Reference) (OtherComp :type Primitive%20Component%20Object%20Reference) (OtherBodyIndex :type Integer))
  (bind _asbp_third_person_character (Utilities|Casting|CastToBP_ThirdPersonCharacter OtherActor))
  (Variables|/Game/ThirdPerson/Blueprints/BP_ThirdPersonCharacter.BP_ThirdPersonCharacter_C|SetCurrentBow _asbp_third_person_character 0)
  (Development|PrintString "cannot"))

(event Custom|Hide
  (if (Variables|Default|GetisHiden?)
    (Rendering|SetActorHiddenInGame true)
    (Variables|Default|SetisHiden? false)
    (else
      (Rendering|SetActorHiddenInGame true)
      (Variables|Default|SetisHiden? true))))

(event EventBeginPlay)

(event Collision|EventActorBeginOverlap
  (params (OtherActor :type Actor%20Object%20Reference)))

(event EventTick
  (params (DeltaSeconds :type Float%20%28single-precision%29)))

(fn ConstructionScript)