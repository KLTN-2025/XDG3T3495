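; BP_valve is an interactable water valve that rotates its cylinder and triggers the water rise on a referenced water actor.
; Box overlap registers or clears the valve as the third-person character's CurrentValve, also setting CanInteract and resetting IsOpen.
; ToggleValve flips IsOpen, sets a yaw target and plays or reverses the Valve_Rotate timeline.
; Timeline updates lerp the cylinder's rotation and call StartWaterRise on every tick.
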(event OnComponentBeginOverlap(Box)
  (params (OverlappedComponent :type Primitive%20Component%20Object%20Reference) (OtherActor :type Actor%20Object%20Reference) (OtherComp :type Primitive%20Component%20Object%20Reference) (OtherBodyIndex :type Integer) (bFromSweep :type Boolean) (SweepResult :type Hit%20Result%20Structure%20%28by%20ref%29))
  (Variables|Default|SetCanInteract true)
  (bind _asbp_third_person_character (Utilities|Casting|CastToBP_ThirdPersonCharacter OtherActor))
  (Variables|/Game/ThirdPerson/Blueprints/BP_ThirdPersonCharacter.BP_ThirdPersonCharacter_C|SetCurrentValve _asbp_third_person_character self)
  (Variables|Default|SetIsOpen false))

(event OnComponentEndOverlap(Box)
  (params (OverlappedComponent :type Primitive%20Component%20Object%20Reference) (OtherActor :type Actor%20Object%20Reference) (OtherComp :type Primitive%20Component%20Object%20Reference) (OtherBodyIndex :type Integer))
  (Variables|Default|SetCanInteract false)
  (bind _asbp_third_person_character (Utilities|Casting|CastToBP_ThirdPersonCharacter OtherActor))
  (Variables|/Game/ThirdPerson/Blueprints/BP_ThirdPersonCharacter.BP_ThirdPersonCharacter_C|SetCurrentValve _asbp_third_person_character 0)
  (Variables|Default|SetIsOpen true))

(event Custom|ToggleValve
  (bind _cylinder (Variables|Default|GetCylinder))
  (bind _rotatespeed (Variables|Default|GetRotateSpeed))
  (bind _relativerotation (Variables|/Script/Engine.SceneComponent|GetRelativeRotation _cylinder))
  (bind _yaw (Math|Rotator|BreakRotator _relativerotation))
  (bind _returnvalue (+ _yaw _rotatespeed))
  (bind _returnvalue_2 (Math|Rotator|MakeRotator 0.0 0.0 _returnvalue))
  (if (Variables|Default|GetIsOpen)
    (Variables|Default|SetIsOpen false)
    (Variables|Default|SetRotationTarget _returnvalue_2)
    (bind _rotationalpha (Timeline|Valve_Rotate Reverse)
      (:Update
        (Transformation|SetRelativeRotation (Variables|Default|GetCylinder) (Math|Rotator|Lerp(Rotator) (Transformation|GetActorRotation (Components|GetOwner (Variables|Default|GetCylinder))) (Variables|Default|GetRotationTarget) _rotationalpha) false false)
        (bind _output_get (Variables|Default|SetWaterRef (Variables|Default|GetWaterRef)))
        (Default|StartWaterRise _output_get)))
    (else
      (Variables|Default|SetIsOpen true)
      (Variables|Default|SetRotationTarget _returnvalue_2)
      (Timeline|Valve_Rotate Play))))

(event EventBeginPlay)

(event Collision|EventActorBeginOverlap
  (params (OtherActor :type Actor%20Object%20Reference)))

(fn ConstructionScript)