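; BP_water is a water actor that rises to a target Height when its StartWaterRise event is called.
; The event plays the TL_movewater timeline, whose WaterHeight track drives a swept vector lerp of the actor's Z while keeping X and Y.
; The lerp starts from the current location on every update, so motion compounds rather than following the curve directly.
; BeginPlay only re-sets the actor's existing location.
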(event Custom|Start%20Water%20Rise
  (bind _returnvalue (Transformation|GetActorLocation))
  (bind _waterheight (Timeline|TL_movewater PlayFromStart)
    (:Update
      (Transformation|SetActorLocation (Math|Vector|Lerp(Vector) _returnvalue (Math|Vector|MakeVector (.X (Math|Vector|BreakVector _returnvalue)) (.Y (Math|Vector|BreakVector _returnvalue)) (Variables|Default|GetHeight)) _waterheight) true false))))

(event EventBeginPlay
  (Transformation|SetActorLocation (Transformation|GetActorLocation) false false))

(event Collision|EventActorBeginOverlap
  (params (OtherActor :type Actor%20Object%20Reference)))

(event EventTick
  (params (DeltaSeconds :type Float%20%28single-precision%29)))

(fn ConstructionScript)