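; BP_Door is a door that opens once the player has collected enough items.
; Each collectitem call increments a counter, and reaching the configured maximum fires OpenDoor through a DoOnce so it triggers only once.
; OpenDoor plays a timeline that lerps the Door component's relative location straight up to raise it.
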(event Custom|Open%20Door
  (bind _door_lift (Timeline|OpenDoorAnim Play)
    (:Update
      (Transformation|SetRelativeLocation (Variables|Default|Getdoor) (Math|Vector|Lerp(Vector) "0, 0, 0" "0.000000,0.000000,426.000000" _door_lift) false false))))

(event Custom|collect%20item
  (Math|Integer|IncrementInt (Variables|Default|GetCurrentItemCollect)
    (:%20%20
      (if (>= (Variables|Default|GetCurrentItemCollect) (Variables|Default|GetMaxItemCollect))
        (Utilities|FlowControl|DoOnce false
          (:Completed
            (CallFunction|OpenDoor)))))))

(event EventBeginPlay)

(event Collision|EventActorBeginOverlap
  (params (OtherActor :type Actor%20Object%20Reference)))

(event EventTick
  (params (DeltaSeconds :type Float%20%28single-precision%29)))

(fn ConstructionScript)